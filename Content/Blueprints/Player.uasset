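; Player character Blueprint that handles movement, jumping, mouse look, and attack and block states from input.
; Mouse X yaws the controller, while Mouse Y pitches the spring arm and clamps its angle.
; Attack sets a flag cleared by a fixed delay, and Block sets one while held.
; Either flag suppresses movement and new attacks, attacking prevents blocking, and jumping only requires being on the ground.
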(event `InputAxisKey|MouseY`
  (params (AxisValue :type "Float (single-precision)"))
  (`SceneComponent.K2_AddLocalRotation` (`self.SpringArm`) (`KismetMathLibrary.MakeRotator` 0.0 AxisValue) false false)
  (`SceneComponent.K2_SetRelativeRotation` (`self.SpringArm`) (`KismetMathLibrary.MakeRotator` 0.0 (`KismetMathLibrary.ClampAngle` (.pitch (`SpringArmComponent.GetTargetRotation` (`self.SpringArm`))) 45.0 40.0)) false false))

(event `InputAction|Jump`
  (params (Key :type "Key Structure"))
  (:`Pressed`
    (if (`NavMovementComponent.IsMovingOnGround` (`self.CharacterMovement`))
      (`self.Jump`))))

(event `InputAxisKey|MouseX`
  (params (AxisValue :type "Float (single-precision)"))
  (`self.AddControllerYawInput` AxisValue))

(event `InputAxis|Move_LeftRight`
  (params (AxisValue :type "Float (single-precision)"))
  (if (not (or (`self.attacking`) (`self.blocking`)))
    (`self.AddMovementInput` (`self.GetActorRightVector`) AxisValue)))

(event `InputAction|Attack`
  (params (Key :type "Key Structure"))
  (:`Pressed`
    (if (not (or (`self.attacking`) (`self.blocking`)))
      (set `self.attacking` true)
      (`KismetSystemLibrary.Delay` 1.5)
      (set `self.attacking` false))))

(event `InputAxis|Move_ForwardsBack`
  (params (AxisValue :type "Float (single-precision)"))
  (if (not (or (`self.attacking`) (`self.blocking`)))
    (`self.AddMovementInput` (`self.GetActorForwardVector`) AxisValue)))

(event `InputAction|Block`
  (params (Key :type "Key Structure"))
  (:`Pressed`
    (if (not (`self.attacking`))
      (set `self.blocking` true)))
  (:`Released`
    (set `self.blocking` false)))

(fn `UserConstructionScript`)